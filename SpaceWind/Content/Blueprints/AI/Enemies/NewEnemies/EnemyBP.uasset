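; EnemyBP is an enemy that chases the player and damages them on contact, destroying itself in the process.
; PawnSensing locks the first PlayerCharacterBP seen as Target while none is valid.
; Tick moves it toward Target with yaw-only movement input and lerped rotation, both only while farther than AttackDistance.
; A Box overlap with the player subtracts Damage directly from Health, then destroys the enemy.
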(event OnSeePawn(PawnSensing)
  (params (Pawn :type Pawn%20Object%20Reference))
  (Variables|Default|GetTarget
    (:then)
    (:else
      (bind _asplayer_character_bp (Utilities|Casting|CastToPlayerCharacterBP Pawn))
      (Variables|Default|SetTarget _asplayer_character_bp))))

(event OnComponentBeginOverlap(Box)
  (params (OverlappedComponent :type Primitive%20Component%20Object%20Reference) (OtherActor :type Actor%20Object%20Reference) (OtherComp :type Primitive%20Component%20Object%20Reference) (OtherBodyIndex :type Integer) (bFromSweep :type Boolean) (SweepResult :type Hit%20Result%20Structure%20%28by%20ref%29))
  (bind _asplayer_character_bp (Utilities|Casting|CastToPlayerCharacterBP OtherActor))
  (Variables|/Game/Blueprints/Player/PlayerCharacterBP.PlayerCharacterBP_C|SetHealth _asplayer_character_bp (- (Variables|/Game/Blueprints/Player/PlayerCharacterBP.PlayerCharacterBP_C|GetHealth _asplayer_character_bp) (Variables|Default|GetDamage)))
  (Actor|DestroyActor))

(event EventTick
  (params (DeltaSeconds :type Float%20%28single-precision%29))
  (bind _target (Variables|Default|GetTarget)
    (:then
      (if (> (Transformation|GetDistanceTo _target) (Variables|Default|GetAttackDistance))
        (Pawn|Input|AddMovementInput (Math|Rotator|GetRotationXVector (Math|Rotator|MakeRotator 0.0 0.0 (.yaw (Math|Rotator|FindLookatRotation (Transformation|GetActorLocation) (+ (Transformation|GetActorLocation _target) "0, 0,0.000000"))))) 1.0 false)
        (Transformation|SetActorRotation (Math|Rotator|Lerp(Rotator) (Transformation|GetActorRotation) (Math|Rotator|MakeRotator 0.0 0.0 (.yaw (Math|Rotator|FindLookatRotation (Transformation|GetActorLocation) (+ (Transformation|GetActorLocation _target) "0, 0,0.000000")))) 0.1 true))))
    (:else)))

(fn ConstructionScript)