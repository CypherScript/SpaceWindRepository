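; CombatTrigger is a trigger actor that shifts global time dilation when the player enters or leaves it.
; Both overlaps restart the SlowPlayer timeline, whose update lerps time dilation toward GameSpeed using its TransitionSpeed track.
; Exit sets GameSpeed to normal; entry assigns it to itself, so the slow value is not restored on re-entry.
; An EnemyPrompt widget creation chain is left unconnected.
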(event EventBeginPlay)

(event Collision|EventActorBeginOverlap
  (params (OtherActor :type Actor%20Object%20Reference))
  (Utilities|Casting|CastToPlayerCharacterBP OtherActor)
  (Variables|Default|SetGameSpeed (Variables|Default|GetGameSpeed))
  (Components|Timeline|PlayfromStart (Variables|Default|GetSlowPlayer)))

(event EventTick
  (params (DeltaSeconds :type Float%20%28single-precision%29)))

(event Collision|EventActorEndOverlap
  (params (OtherActor :type Actor%20Object%20Reference))
  (Utilities|Casting|CastToPlayerCharacterBP OtherActor)
  (Variables|Default|SetGameSpeed 1.0)
  (Components|Timeline|PlayfromStart (Variables|Default|GetSlowPlayer)))

(fn ConstructionScript)