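; TransitionTrigger is a trigger actor that moves the player character between two spline paths, SplineA and SplineB.
; On player overlap it caches the character and clears the game instance's navigating flag.
; If the player is on SplineA, it switches them to SplineB and opens a navigation screen widget.
; ToggleSpline swaps the cached player's path, and leaving the sphere clears only the overlap flag.
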(event OnComponentEndOverlap(Sphere)
  (params (OverlappedComponent :type Primitive%20Component%20Object%20Reference) (OtherActor :type Actor%20Object%20Reference) (OtherComp :type Primitive%20Component%20Object%20Reference) (OtherBodyIndex :type Integer))
  (Utilities|Casting|CastToPlayerCharacterBP OtherActor)
  (Variables|Default|SetisOverlappingPlayer false))

(event Custom|ToggleSpline
  (bind _splinea (Variables|Default|GetSplineA))
  (bind _playerreference (Variables|Default|GetPlayerReference))
  (if (== (Variables|/Game/Blueprints/Player/PlayerCharacterBP.PlayerCharacterBP_C|GetPlayerPath _playerreference) _splinea)
    (Variables|/Game/Blueprints/Player/PlayerCharacterBP.PlayerCharacterBP_C|SetPlayerPath _playerreference (Variables|Default|GetSplineB))
    (else
      (Variables|/Game/Blueprints/Player/PlayerCharacterBP.PlayerCharacterBP_C|SetPlayerPath _playerreference _splinea))))

(event EventBeginPlay)

(event Collision|EventActorBeginOverlap
  (params (OtherActor :type Actor%20Object%20Reference))
  (bind _asplayer_character_bp (Utilities|Casting|CastToPlayerCharacterBP OtherActor))
  (Variables|Default|SetPlayerReference _asplayer_character_bp)
  (Variables|Default|SetisOverlappingPlayer true)
  (bind _asspace_wind_game_instance (Utilities|Casting|CastToSpaceWindGameInstance (Game|GetGameInstance)))
  (Variables|/Game/Blueprints/GameInstance/SpaceWindGameInstance.SpaceWindGameInstance_C|SetIsPlayerNavigating _asspace_wind_game_instance false)
  (if (== (Variables|/Game/Blueprints/Player/PlayerCharacterBP.PlayerCharacterBP_C|GetPlayerPath (Variables|Default|GetPlayerReference)) (Variables|Default|GetSplineA))
    (Variables|/Game/Blueprints/Player/PlayerCharacterBP.PlayerCharacterBP_C|SetPlayerPath (Variables|Default|GetPlayerReference) (Variables|Default|GetSplineB))
    (bind _returnvalue (UserInterface|CreateWidget "/Game/Blueprints/UI_Screens/NavigationScreenBP.NavigationScreenBP_C"))
    (UserInterface|Viewport|AddtoViewport _returnvalue 0)))

(event EventTick
  (params (DeltaSeconds :type Float%20%28single-precision%29)))

(fn ConstructionScript)