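; Player character for a sailboat game that snaps to the PlayerPath spline on start, shows HUD and navigation prompt, and handles pausing.
; Space opens six navigation screens in sequence via the NavPuzzle counter.
; Overlapping a TransitionTrigger stores it and clears IsNavigating, so Space toggles its spline before opening the next screen.
; Tick sets the global Music audio parameter every frame; the timeline code for moving along the spline is unconnected.
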(event EventBeginPlay
  (Transformation|SetWorldLocation (Variables|Collision|GetCapsuleComponent) (Spline|FindLocationClosesttoWorldLocation (Variables|/Game/Blueprints/Path/PlayerPathBP.PlayerPathBP_C|GetSpline (Variables|Default|GetPlayerPath)) (Transformation|GetWorldLocation (Variables|Collision|GetCapsuleComponent)) "World") false true)
  (bind _returnvalue (UserInterface|CreateWidget "/Game/Blueprints/Player/HUD/HUD.HUD_C"))
  (UserInterface|Viewport|AddtoPlayerScreen _returnvalue)
  (bind _returnvalue_2 (UserInterface|CreateWidget "/Game/Blueprints/Player/HUD/EnableNavigationPrompt.EnableNavigationPrompt_C"))
  (bind _output_get (Variables|Default|SetNavPromptRef _returnvalue_2))
  (UserInterface|Viewport|AddtoViewport _output_get 0))

(event EventTick
  (params (DeltaSeconds :type Float%20%28single-precision%29))
  (Class|FMODBlueprintStatics|SetGlobalParameterbyName "Music" 3.0))

(event Collision|EventActorBeginOverlap
  (params (OtherActor :type Actor%20Object%20Reference))
  (bind _astransition_trigger (Utilities|Casting|CastToTransitionTrigger OtherActor))
  (Variables|Default|SetSplineTransitionReference _astransition_trigger)
  (Variables|Default|SetIsNavigating false))

(event Input|ActionEvents|InputActionPause
  (params (Key :type Key%20Structure))
  (:Pressed
    (CallFunction|PausedMenu)))

(event Input|KeyboardEvents|W
  (params (Key :type Key%20Structure)))

(event Input|KeyboardEvents|SpaceBar
  (params (Key :type Key%20Structure))
  (bind _splinetransitionreference (Variables|Default|GetSplineTransitionReference))
  (:Pressed
    (if (Variables|Default|GetIsNavigating)
      (switch int (Variables|Default|GetNavPuzzle) :!label _label
        (:0
          (bind _returnvalue (UserInterface|CreateWidget "/Game/Blueprints/UI_Screens/NavigationScreenBP.NavigationScreenBP_C" :!label _label_2))
          (UserInterface|Viewport|AddtoViewport _returnvalue 0))
        (:1
          (bind _returnvalue_2 (UserInterface|CreateWidget "/Game/Blueprints/UI_Screens/NavigationScreenBP2.NavigationScreenBP2_C"))
          (UserInterface|Viewport|AddtoViewport _returnvalue_2 0))
        (:2
          (bind _returnvalue_3 (UserInterface|CreateWidget "/Game/Blueprints/UI_Screens/NavigationScreenBP3.NavigationScreenBP3_C"))
          (UserInterface|Viewport|AddtoViewport _returnvalue_3 0))
        (:3
          (bind _returnvalue_4 (UserInterface|CreateWidget "/Game/Blueprints/UI_Screens/NavigationScreenBP4.NavigationScreenBP4_C"))
          (UserInterface|Viewport|AddtoViewport _returnvalue_4 0))
        (:4
          (bind _returnvalue_5 (UserInterface|CreateWidget "/Game/Blueprints/UI_Screens/NavigationScreenBP5.NavigationScreenBP5_C"))
          (UserInterface|Viewport|AddtoViewport _returnvalue_5 0))
        (:5
          (bind _returnvalue_6 (UserInterface|CreateWidget "/Game/Blueprints/UI_Screens/NavigationScreenBP6.NavigationScreenBP6_C"))
          (UserInterface|Viewport|AddtoViewport _returnvalue_6 0)))
      (Variables|Default|SetNavPuzzle (+ (Variables|Default|GetNavPuzzle) 1))
      (Variables|Default|SetIsNavigating true)
      (Widget|RemovefromParent (Variables|Default|GetNavPromptRef))
      (else
        (Utilities|IsValid _splinetransitionreference
          (:Is%20Valid
            (if (Variables|/Game/Blueprints/Triggers/TransitionTrigger.TransitionTrigger_C|GetisOverlappingPlayer _splinetransitionreference)
              (Default|ToggleSpline _splinetransitionreference)
              (goto _label)))
          (:Is%20Not%20Valid
            (goto _label_2)))))))

(fn ConstructionScript)

(fn PausedMenu
  (Game|SetGamePaused true)
  (Utilities|IsValid (Variables|Default|GetPauseMenu)
    (:Is%20Valid
      _)
    (:Is%20Not%20Valid
      (bind _returnvalue (UserInterface|CreateWidget "/Game/Blueprints/Player/HUD/PauseMenu.PauseMenu_C" (Game|GetPlayerController 0)))
      (Variables|Default|SetPauseMenu _returnvalue)))
  (UserInterface|Viewport|AddtoViewport (Variables|Default|GetPauseMenu) 0)
  (Input|SetInputModeUIOnly (Game|GetPlayerController 0) (Variables|Default|GetPauseMenu) "DoNotLock")
  (Variables|/Script/Engine.PlayerController|SetbShowMouseCursor (Game|GetPlayerController 0) true))

(fn Un-Paused
  (bind _returnvalue (Game|GetPlayerController 0))
  (Game|SetGamePaused false)
  (Viewport|RemoveAllWidgets)
  (Input|SetInputModeGameOnly _returnvalue)
  (Variables|/Script/Engine.PlayerController|SetbShowMouseCursor _returnvalue false))