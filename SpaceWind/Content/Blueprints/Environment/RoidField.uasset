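; RoidField is an environment Blueprint that scatters an asteroid field around its origin as instances of one InstancedStaticMesh.
; The construction script adds instances in a loop driven by TotalRoid, each at a random direction and distance between MinDistance and MaxDistance, forming a spherical shell.
; Each gets random rotation and uniform scale within configurable limits.
; Randomness is unseeded, so the layout changes whenever construction reruns; the event graph is inactive.
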(event EventBeginPlay)

(event Collision|EventActorBeginOverlap
  (params (OtherActor :type Actor%20Object%20Reference)))

(event EventTick
  (params (DeltaSeconds :type Float%20%28single-precision%29)))

(fn ConstructionScript
  (for _index (range 0 (Variables|Default|GetTotalRoid))
    (Components|InstancedStaticMesh|AddInstance (Variables|Default|GetInstancedStaticMesh) (Math|Transform|MakeTransform (* (Math|Random|RandomUnitVector) (Math|Random|RandomFloatinRange (Variables|Default|GetMin%20Distance) (Variables|Default|GetMax%20Distance))) (Math|Random|RandomRotator false) (Math|Conversions|ToVector(Float) (* (Math|Random|RandomFloatinRange (Variables|Default|GetMin%20Scale) (Variables|Default|GetMax%20Scale)) (Variables|Default|GetScale%20mulitplier)))))))